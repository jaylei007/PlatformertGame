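; Swimming NPC interactable that displays a text message in the player's sign widget when interacted with.
; Interaction runs the parent logic, sets the sign text and plays the widget's blend-in animation, while ending interaction plays the blend-out.
; The construction script applies a selectable color variant by setting a material from the Colors list on the skeletal mesh's second slot.
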(event `self.OnInteract`
  (bind _signwidget (`/Game/PlatformerDevelopmentKit/UI/Widgets/Main_Widget.SignWidget` (`/Game/PlatformerDevelopmentKit/Characters/Player/Blueprints/BP_Rabbit.MainWidgetReference` (`self.PlayerReference`))))
  (`parent.OnInteract`)
  (`TextBlock.SetText` (`/Game/PlatformerDevelopmentKit/UI/Widgets/Sign_Widget.SignText` _signwidget) (`self.SignText`))
  (`UserWidget.PlayAnimation` _signwidget (`/Game/PlatformerDevelopmentKit/UI/Widgets/Sign_Widget.BlendIn` _signwidget) 0.0 1 "Forward" 1.0 false))

(event `self.OnInteractEnd`
  (bind _signwidget (`/Game/PlatformerDevelopmentKit/UI/Widgets/Main_Widget.SignWidget` (`/Game/PlatformerDevelopmentKit/Characters/Player/Blueprints/BP_Rabbit.MainWidgetReference` (`self.PlayerReference`))))
  (`UserWidget.PlayAnimation` _signwidget (`/Game/PlatformerDevelopmentKit/UI/Widgets/Sign_Widget.BlendOut` _signwidget) 0.0 1 "Forward" 1.0 false))

(fn `UserConstructionScript`
  (`parent.UserConstructionScript`)
  (`PrimitiveComponent.SetMaterial` (`self.SK_Interactable`) 1 (`|GetArrayItem` (`self.Colors`) (`self.Color`))))