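; Wandering jellyfish hazard that swims between random nearby points and shocks the rabbit player on contact.
; Tick moves it forward with sweep while turning toward its target; on arrival it picks another, using sphere traces to reject blocked paths and falling back to its spawn point.
; Capsule overlap triggers a DoOnce-gated hit: physics knockback, lightning effect, heart loss and a timed recovery.
; BeginPlay randomizes scale and animation rate for variety.
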(event `self.ReceiveTick`
  (params (DeltaSeconds :type "Float (single-precision)"))
  (`self.K2_AddActorLocalOffset` (`KismetMathLibrary.MakeVector` (* (`self.Current forward speed`) DeltaSeconds)) true) ; Sweep plane forwards
  (`self.K2_SetActorRotation` (`KismetMathLibrary.RInterpTo` (`self.K2_GetActorRotation`) (`KismetMathLibrary.FindLookAtRotation` (`self.K2_GetActorLocation`) (`self.LocationToSwim`)) DeltaSeconds 2.0))
  (if (`KismetMathLibrary.NearlyEqual_TransformTransform` (`KismetMathLibrary.MakeTransform` (`self.K2_GetActorLocation`)) (`KismetMathLibrary.MakeTransform` (`self.LocationToSwim`)) 50.0 50.0 50.0)
    (`self.SwimToLocation`)))

(event `self.ReceiveBeginPlay`
  (bind _returnvalue (`KismetMathLibrary.RandomFloatInRange` 1.0 2.0))
  (set `self.OriginLocation` (`self.K2_GetActorLocation`))
  (`self.SetActorScale3D` (`KismetMathLibrary.MakeVector` _returnvalue _returnvalue _returnvalue))
  (`SkeletalMeshComponent.SetPlayRate` (`self.SkeletalMesh`) (`KismetMathLibrary.RandomFloatInRange` 0.9 1.1))
  (`self.SwimToLocation`)
  (`KismetSystemLibrary.Delay` 1.0)
  (bind _asbp_rabbit (cast `/Game/PlatformerDevelopmentKit/Characters/Player/Blueprints/BP_Rabbit` (`GameplayStatics.GetPlayerCharacter` 0)))
  (set `self.RabbitReference` _asbp_rabbit))

(event `SwimToLocation`
  (set `self.LocationToSwim` (`KismetMathLibrary.RandomPointInBoundingBox` (`SceneComponent.K2_GetComponentLocation` (`self.DefaultSceneRoot`)) (500.0 500.0 200.0)) :!label _label)
  (bind (_outhit _returnvalue) (`KismetSystemLibrary.SphereTraceSingle` (`self.K2_GetActorLocation`) (`self.LocationToSwim`) 50.0 "TraceTypeQuery5" false (`|MakeArray` (`self.RabbitReference`) self :!type "Actor Object Reference")))
  (if _returnvalue
    (if (< (`self.TriesAmount`) 4)
      (`/Engine/EditorBlueprintResources/StandardMacros.IncrementInt` (`self.TriesAmount`)
        (:`  `
          (goto _label)))
      (else
        (set `self.LocationToSwim` (`self.OriginLocation`))
        (set `self.TriesAmount` 0)))))

(event `CanBeDamagedAgainPlayer`
  (bind _playerreference (`self.PlayerReference`))
  (bind _playerreference_2 (`self.PlayerReference`))
  (bind _playerreference_3 (`self.PlayerReference`))
  (bind _playerreference_4 (`self.PlayerReference`))
  (bind _capsulecomponent (`Character.CapsuleComponent` _playerreference_3))
  (goto _label_2 :!via `Reset`))

(event `self.Capsule.OnComponentBeginOverlap`
  (params (OverlappedComponent :type "PrimitiveComponent Object Reference") (OtherActor :type "Actor Object Reference") (OtherComp :type "PrimitiveComponent Object Reference") (OtherBodyIndex :type Integer) (bFromSweep :type Boolean) (SweepResult :type "HitResult Structure (by ref)"))
  (bind _playerreference (`self.PlayerReference`))
  (bind _playerreference_2 (`self.PlayerReference`))
  (bind _playerreference_3 (`self.PlayerReference`))
  (bind _playerreference_4 (`self.PlayerReference`))
  (bind _capsulecomponent (`Character.CapsuleComponent` _playerreference_3))
  (bind _asbp_rabbit (cast `/Game/PlatformerDevelopmentKit/Characters/Player/Blueprints/BP_Rabbit` OtherActor))
  (bind _output_get (set `self.PlayerReference` _asbp_rabbit))
  (`/Engine/EditorBlueprintResources/StandardMacros.DoOnce` false :!label _label_2
    (:`Completed`
      (if (`/Game/PlatformerDevelopmentKit/Characters/Player/Blueprints/BP_Rabbit.IsHanging?` (`self.PlayerReference`))
        (`/Game/PlatformerDevelopmentKit/Characters/Player/Blueprints/BP_Rabbit.GetOffLedge` (`self.PlayerReference`)))
      (`self.DisableInput` _output_get (`GameplayStatics.GetPlayerController` 0))
      (`PrimitiveComponent.SetSimulatePhysics` (`Character.CapsuleComponent` (`self.PlayerReference`)) true)
      (`PrimitiveComponent.AddImpulse` _capsulecomponent (* (`self.GetActorForwardVector` _playerreference_3) -800.0) "None" true)
      (`PrimitiveComponent.AddAngularImpulseInDegrees` _capsulecomponent (180.0 180.0 180.0) "None" true)
      (set `/Game/PlatformerDevelopmentKit/Characters/Player/Blueprints/BP_Rabbit.CharacterCondition` "NewEnumerator0" _playerreference)
      (`GameplayStatics.SpawnEmitterAttached` "/Game/PlatformerDevelopmentKit/Interactables/Particles/PS_Lightning.PS_Lightning" (`Character.Mesh` _playerreference) "spine1" (0.0 0.0 0.0) (struct) (1.0 1.0 1.0) "SnapToTarget")
      (`/Game/PlatformerDevelopmentKit/UI/Widgets/Main_Widget.UpdateHearts` (`/Game/PlatformerDevelopmentKit/Characters/Player/Blueprints/BP_Rabbit.MainWidgetReference` (`self.PlayerReference`)) -1)
      (if (<= (`/Game/PlatformerDevelopmentKit/Characters/Player/Blueprints/BP_Rabbit.CurrentHealth` (`self.PlayerReference`)) 0)
        (set `/Game/PlatformerDevelopmentKit/Characters/Player/Blueprints/BP_Rabbit.CharacterCondition` "NewEnumerator1" _playerreference_4)
        (`self.DisableInput` _playerreference_4 (`GameplayStatics.GetPlayerController` 0))
        (`KismetSystemLibrary.Delay` 1.6)
        (`self.CanBeDamagedAgainPlayer`)
        (else
          (`KismetSystemLibrary.Delay` 1.6)
          (`self.CanBeDamagedAgainPlayer`)))
      (`MovementComponent.StopMovementImmediately` (`Character.CharacterMovement` _playerreference_2))
      (`PrimitiveComponent.SetSimulatePhysics` (`Character.CapsuleComponent` _playerreference_2) false))))

(fn `UserConstructionScript`)