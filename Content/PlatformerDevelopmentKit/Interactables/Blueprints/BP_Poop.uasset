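; BP_Poop is a collectible pickup that adds to the rabbit player's poop count.
; When BP_Rabbit overlaps its sphere, it disables the sphere's collision, increments PoopAmount, then refreshes and reveals the poop counter on the main widget.
; It spawns a crumb particle effect and plays a pickup animation on the skeletal mesh, then destroys itself after a short delay.
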(event `self.Sphere.OnComponentBeginOverlap`
  (params (OverlappedComponent :type "PrimitiveComponent Object Reference") (OtherActor :type "Actor Object Reference") (OtherComp :type "PrimitiveComponent Object Reference") (OtherBodyIndex :type Integer) (bFromSweep :type Boolean) (SweepResult :type "HitResult Structure (by ref)"))
  (bind _asbp_rabbit (cast `/Game/PlatformerDevelopmentKit/Characters/Player/Blueprints/BP_Rabbit` OtherActor))
  (`PrimitiveComponent.SetCollisionResponseToAllChannels` (`self.Sphere`) "ECR_Ignore")
  (set `/Game/PlatformerDevelopmentKit/Characters/Player/Blueprints/BP_Rabbit.PoopAmount` (+ (`/Game/PlatformerDevelopmentKit/Characters/Player/Blueprints/BP_Rabbit.PoopAmount` _asbp_rabbit) 1) _asbp_rabbit)
  (bind _mainwidgetreference (`/Game/PlatformerDevelopmentKit/Characters/Player/Blueprints/BP_Rabbit.MainWidgetReference` _asbp_rabbit))
  (`/Game/PlatformerDevelopmentKit/UI/Widgets/Main_Widget.UpdatePoop` _mainwidgetreference)
  (`Widget.SetVisibility` (`/Game/PlatformerDevelopmentKit/UI/Widgets/Main_Widget.PoopBox` _mainwidgetreference) "SelfHitTestInvisible")
  (`GameplayStatics.SpawnEmitterAtLocation` "/Game/PlatformerDevelopmentKit/Interactables/Particles/PS_PoopCrums.PS_PoopCrums" (`SceneComponent.K2_GetComponentLocation` (`self.Sphere`)))
  (`SkeletalMeshComponent.PlayAnimation` (`self.SK_Coin`) "/Game/PlatformerDevelopmentKit/Interactables/Animations/PoopPickup_Anim.PoopPickup_Anim" false)
  (`KismetSystemLibrary.Delay` 0.583)
  (`self.K2_DestroyActor`))

(fn `UserConstructionScript`)