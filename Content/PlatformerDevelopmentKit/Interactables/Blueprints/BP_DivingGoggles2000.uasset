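; BP_DivingGoggles2000 is an obtainable item that equips diving goggles and sets the player's oxygen stats.
; When obtained, its PlayItemAnimationwhenObtained event adds a collision-free goggles static mesh to the player and attaches it to the GogglesSocket on the character mesh.
; It then overwrites the player's maximum oxygen, current oxygen and regeneration rate with fixed values.
; The construction script only calls the parent's.
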(event `self.PlayItemAnimationWhenObtained`
  (bind _playerreference (`self.PlayerReference`))
  (bind _playerreference_2 (`self.PlayerReference`))
  (bind _returnvalue (`AddComponent|NODE_AddStaticMeshComponent-0` :`self` _playerreference_2))
  (`StaticMeshComponent.SetStaticMesh` _returnvalue "/Game/PlatformerDevelopmentKit/Interactables/Meshes/SM_Goggles.SM_Goggles")
  (`PrimitiveComponent.SetCollisionEnabled` _returnvalue "NoCollision")
  (`SceneComponent.K2_AttachToComponent` _returnvalue (`Character.Mesh` _playerreference_2) "GogglesSocket" "KeepRelative" "KeepRelative" "KeepRelative" true)
  (set `/Game/PlatformerDevelopmentKit/Characters/Player/Blueprints/BP_Rabbit.MaxOxygen` 120.0 _playerreference)
  (set `/Game/PlatformerDevelopmentKit/Characters/Player/Blueprints/BP_Rabbit.CurrentOxygen` 120.0 _playerreference)
  (set `/Game/PlatformerDevelopmentKit/Characters/Player/Blueprints/BP_Rabbit.OxygenRegenrate` 0.4 _playerreference))

(fn `UserConstructionScript`
  (`parent.UserConstructionScript`))