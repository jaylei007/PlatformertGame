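; BP_RevealAbility is the player's reveal ability, publishing the player's position for materials to read.
; On BeginPlay it adds a tiny sphere component to the player, sets it to ignore all collision channels and attaches it to the mesh's head socket.
; Each Tick it writes the sphere's world location to the PlayerPosition vector in the PC_PlayerPosition material parameter collection.
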(event `self.ReceiveBeginPlay`
  (bind _playerreference (`self.PlayerReference`))
  (bind _returnvalue (`AddComponent|NODE_AddSphereComponent-0` :`self` _playerreference :`RelativeTransform` (`KismetMathLibrary.MakeTransform` (0.0 0.0 3.5) (struct :`Pitch` 90.0 :`Roll` -90.0) (0.003 0.003 0.003))))
  (set `self.Sphere` _returnvalue)
  (`PrimitiveComponent.SetCollisionResponseToAllChannels` _returnvalue "ECR_Ignore")
  (`SceneComponent.K2_AttachToComponent` _returnvalue (`Character.Mesh` _playerreference) "head" "KeepRelative" "KeepRelative" "KeepRelative" true))

(event `self.ReceiveTick`
  (params (DeltaSeconds :type "Float (single-precision)"))
  (bind _sphere (`self.Sphere`))
  (`/Engine/EditorBlueprintResources/StandardMacros.IsValid` _sphere
    (:`Is Valid`
      (`KismetMaterialLibrary.SetVectorParameterValue` "/Game/PlatformerDevelopmentKit/Base/Materials/PC_PlayerPosition.PC_PlayerPosition" "PlayerPosition" (`KismetMathLibrary.Conv_VectorToLinearColor` (`SceneComponent.K2_GetComponentLocation` _sphere))))))

(fn `UserConstructionScript`)