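; BP_Cage is a breakable cage interactable that the player destroys by hitting it with thrown poop projectiles.
; Each BP_PoopThrown hit on the Destructible component lowers Health and spawns a star particle burst at the impact point.
; At zero Health the component takes damage to fracture, ignores all collision, and closes a Gate that blocks further hit processing.
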(event `LockFurtherInteraction`
  (bind _destructible (`self.Destructible`))
  (bind _returnvalue (`SceneComponent.K2_GetComponentLocation` _destructible))
  (goto _label :!via `Close`))

(event `self.Destructible.OnComponentHit`
  (params (HitComponent :type "PrimitiveComponent Object Reference") (OtherActor :type "Actor Object Reference") (OtherComp :type "PrimitiveComponent Object Reference") (NormalImpulse :type "Vector Structure") (Hit :type "HitResult Structure (by ref)"))
  (bind _destructible (`self.Destructible`))
  (bind _returnvalue (`SceneComponent.K2_GetComponentLocation` _destructible))
  (`/Engine/EditorBlueprintResources/StandardMacros.Gate` false :!label _label
    (:`Exit`
      (cast `/Game/PlatformerDevelopmentKit/Interactables/Blueprints/BP_PoopThrown` OtherActor)
      (set `self.Health` (- (`self.Health`) 1))
      (`GameplayStatics.SpawnEmitterAtLocation` "/Game/PlatformerDevelopmentKit/Interactables/Particles/PS_Stars.PS_Stars" (`.ImpactPoint` (`GameplayStatics.BreakHitResult` Hit)))
      (if (<= (`self.Health`) 0)
        (`DestructibleComponent.ApplyDamage` _destructible 10.0 _returnvalue _returnvalue 50.0)
        (`PrimitiveComponent.SetCollisionResponseToAllChannels` (`self.Destructible`) "ECR_Ignore")
        (`self.LockFurtherInteraction`)))))

(fn `UserConstructionScript`)