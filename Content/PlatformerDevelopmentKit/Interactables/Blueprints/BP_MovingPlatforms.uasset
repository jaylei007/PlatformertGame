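; BP_MovingPlatforms is an interactable actor with two platforms that move along animated paths.
; On BeginPlay, the PlatformMovement timeline plays and sets each platform's relative location from its own track, without sweep.
; The construction script zeroes each platform's world roll and pitch while keeping its yaw, so both stay level however the actor is rotated.
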(event `self.ReceiveBeginPlay`
  (bind (_direction _platform01 _platform02) (`Timeline|PlatformMovement`)
    (:`Update`
      (`SceneComponent.K2_SetRelativeLocation` (`self.Platform01`) _platform01 false false)
      (`SceneComponent.K2_SetRelativeLocation` (`self.Platform02`) _platform02 false false))))

(fn `UserConstructionScript`
  (bind _platform02 (`self.Platform02`))
  (bind _platform01 (`self.Platform01`))
  (bind (_returnvalue_roll _returnvalue_pitch _returnvalue_yaw) (`KismetMathLibrary.BreakRotator` (`SceneComponent.K2_GetComponentRotation` _platform01)))
  (bind (_returnvalue_roll_2 _returnvalue_pitch_2 _returnvalue_yaw_2) (`KismetMathLibrary.BreakRotator` (`SceneComponent.K2_GetComponentRotation` _platform02)))
  (`SceneComponent.K2_SetWorldRotation` _platform02 (`KismetMathLibrary.MakeRotator` 0.0 0.0 _returnvalue_yaw_2) false false)
  (`SceneComponent.K2_SetWorldRotation` _platform01 (`KismetMathLibrary.MakeRotator` 0.0 0.0 _returnvalue_yaw) false false))