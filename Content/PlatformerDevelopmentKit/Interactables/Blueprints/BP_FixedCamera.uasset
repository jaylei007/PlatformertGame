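; Trigger-volume fixed camera for the platformer that takes over the view while the BP_Rabbit character is inside its box.
; Overlap blends the view to this actor and turns off the rabbit's spring-arm control rotation; leaving reverses both.
; While active, Tick aims the camera at the rabbit and copies its yaw to the player's control rotation.
; Box size and camera transform are applied from variables in the Construction Script.
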(event `self.ReceiveTick`
  (params (DeltaSeconds :type "Float (single-precision)"))
  (if (`self.IsInScope?`)
    (`SceneComponent.K2_SetWorldRotation` (`self.FixedCamera`) (`KismetMathLibrary.FindLookAtRotation` (`SceneComponent.K2_GetComponentLocation` (`self.FixedCamera`)) (`self.K2_GetActorLocation` (`self.RabbitReference`))) false false)
    (`Controller.SetControlRotation` (`GameplayStatics.GetPlayerController` 0) (`KismetMathLibrary.MakeRotator` 0.0 0.0 (.yaw (`SceneComponent.K2_GetComponentRotation` (`self.FixedCamera`)))))))

(event `self.Box.OnComponentBeginOverlap`
  (params (OverlappedComponent :type "PrimitiveComponent Object Reference") (OtherActor :type "Actor Object Reference") (OtherComp :type "PrimitiveComponent Object Reference") (OtherBodyIndex :type Integer) (bFromSweep :type Boolean) (SweepResult :type "HitResult Structure (by ref)"))
  (bind _asbp_rabbit (cast `/Game/PlatformerDevelopmentKit/Characters/Player/Blueprints/BP_Rabbit` OtherActor))
  (set `self.RabbitReference` _asbp_rabbit)
  (`PlayerController.SetViewTargetWithBlend` (`GameplayStatics.GetPlayerController` 0) self 1.0 "VTBlend_Linear" 0.0 false)
  (set `self.IsInScope?` true)
  (set `SpringArmComponent.bUsePawnControlRotation` false (`/Game/PlatformerDevelopmentKit/Characters/Player/Blueprints/BP_Rabbit.SpringArm` (`self.RabbitReference`))))

(event `self.Box.OnComponentEndOverlap`
  (params (OverlappedComponent :type "PrimitiveComponent Object Reference") (OtherActor :type "Actor Object Reference") (OtherComp :type "PrimitiveComponent Object Reference") (OtherBodyIndex :type Integer))
  (bind _returnvalue (`GameplayStatics.GetPlayerController` 0))
  (cast `/Game/PlatformerDevelopmentKit/Characters/Player/Blueprints/BP_Rabbit` OtherActor)
  (`PlayerController.SetViewTargetWithBlend` _returnvalue (`Controller.K2_GetPawn` _returnvalue) 1.0 "VTBlend_Linear" 0.0 false)
  (set `SpringArmComponent.bUsePawnControlRotation` true (`/Game/PlatformerDevelopmentKit/Characters/Player/Blueprints/BP_Rabbit.SpringArm` (`self.RabbitReference`)))
  (set `self.IsInScope?` false))

(fn `UserConstructionScript`
  (`BoxComponent.SetBoxExtent` (`self.Box`) (`self.BoxSize`) true)
  (`SceneComponent.K2_SetRelativeLocation` (`self.FixedCamera`) (`self.CameraPosition`) false false)
  (`SceneComponent.K2_SetRelativeRotation` (`self.FixedCamera`) (`self.CameraRotation`) false false))