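; BP_FlashlightHelmet is an obtainable item that gives the player a helmet with a flashlight and a reveal ability.
; On the obtain event, it adds a helmet static mesh and a spotlight to the player at runtime, attaching both to the character mesh's HelmetSocket.
; It offsets, rotates and configures the spotlight, then spawns BP_RevealAbility with a reference to the player.
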(event `self.PlayItemAnimationWhenObtained`
  (bind _playerreference (`self.PlayerReference`))
  (bind _playerreference_2 (`self.PlayerReference`))
  (bind _returnvalue (`AddComponent|NODE_AddStaticMeshComponent-0` :`self` _playerreference))
  (`StaticMeshComponent.SetStaticMesh` _returnvalue "/Game/PlatformerDevelopmentKit/Interactables/Meshes/SM_FlashlightHelmet.SM_FlashlightHelmet")
  (`SceneComponent.K2_AttachToComponent` _returnvalue (`Character.Mesh` _playerreference) "HelmetSocket" "KeepRelative" "KeepRelative" "KeepRelative" true)
  (bind _returnvalue_2 (`AddComponent|NODE_AddSpotLightComponent-0` :`self` _playerreference_2))
  (`SceneComponent.K2_AttachToComponent` _returnvalue_2 (`Character.Mesh` _playerreference_2) "HelmetSocket" "KeepRelative" "KeepRelative" "KeepRelative" true)
  (`SceneComponent.K2_SetRelativeLocation` _returnvalue_2 (+ (`SceneComponent.RelativeLocation` _returnvalue_2) (0.0 40.0 0.0)) false false)
  (`LightComponent.SetIntensity` _returnvalue_2 200000.0)
  (`SceneComponent.K2_SetRelativeRotation` _returnvalue_2 (struct :`Yaw` 90.0) false false)
  (`LocalLightComponent.SetAttenuationRadius` _returnvalue_2 2000.0)
  (`SpotLightComponent.SetInnerConeAngle` _returnvalue_2 30.0)
  (`|SpawnActorFromClass` "/Game/PlatformerDevelopmentKit/Interactables/Blueprints/BP_RevealAbility.BP_RevealAbility_C" (`KismetMathLibrary.MakeTransform` (0.0 0.0 0.0)) "Undefined" "OverrideRootScale" null (`self.PlayerReference`) null))

(fn `UserConstructionScript`
  (`parent.UserConstructionScript`))