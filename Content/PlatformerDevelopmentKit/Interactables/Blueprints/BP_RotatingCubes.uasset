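; BP_RotatingCubes is a platforming interactable made of two meshes that rotate via a rotating movement component.
; The construction script offsets the meshes in opposite directions along local Y by PlatformDistance and scales both by PlatformSize.
; It also sets a single-axis rotation rate from RotationSpeed, so the component drives all motion and the event graph stays empty.
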(fn `UserConstructionScript`
  (`SceneComponent.K2_AddLocalOffset` (`self.StaticMesh`) (`KismetMathLibrary.MakeVector` 0.0 (`self.PlatformDistance`)) false false)
  (`SceneComponent.K2_AddLocalOffset` (`self.StaticMesh1`) (`KismetMathLibrary.MakeVector` 0.0 (* (`self.PlatformDistance`) -1.0)) false false)
  (`SceneComponent.SetRelativeScale3D` (`self.StaticMesh`) (`self.PlatformSize`))
  (`SceneComponent.SetRelativeScale3D` (`self.StaticMesh1`) (`self.PlatformSize`))
  (set `RotatingMovementComponent.RotationRate` (`KismetMathLibrary.MakeRotator` 0.0 0.0 (`self.RotationSpeed`)) (`self.RotatingMovement`)))