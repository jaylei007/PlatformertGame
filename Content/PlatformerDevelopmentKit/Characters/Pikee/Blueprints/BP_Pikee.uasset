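; BP_Pikee is an AI enemy that damages BP_Rabbit on capsule overlap and takes damage from thrown BP_PoopThrown projectiles.
; Player hits knock the rabbit back, disable input and remove a heart; if the rabbit dies, a living Pikee later teleports to its spawn point.
; Hits on Pikee reduce Health and write AIState to its Blackboard.
; Separate DoOnce gates with delayed resets throttle damage in both directions.
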(event `self.ReceiveBeginPlay`
  (set `self.OriginLocation` (`self.K2_GetActorLocation`))
  (set `self.PikeeBlackboard` (`AIBlueprintHelperLibrary.GetBlackboard` null)))

(event `CanBeDamagedAgainPlayer`
  (bind _playerreference (`self.PlayerReference`))
  (bind _playerreference_2 (`self.PlayerReference`))
  (bind (_returnvalue_x _returnvalue_y) (`KismetMathLibrary.BreakVector` (`self.GetActorForwardVector` (`self.PlayerReference`))))
  (goto _label :!via `Reset`))

(event `self.CapsuleComponent.OnComponentBeginOverlap`
  (params (OverlappedComponent :type "PrimitiveComponent Object Reference") (OtherActor :type "Actor Object Reference") (OtherComp :type "PrimitiveComponent Object Reference") (OtherBodyIndex :type Integer) (bFromSweep :type Boolean) (SweepResult :type "HitResult Structure (by ref)"))
  (bind _playerreference (`self.PlayerReference`))
  (bind _playerreference_2 (`self.PlayerReference`))
  (bind (_returnvalue_x _returnvalue_y) (`KismetMathLibrary.BreakVector` (`self.GetActorForwardVector` (`self.PlayerReference`))))
  (bind _asbp_rabbit (cast `/Game/PlatformerDevelopmentKit/Characters/Player/Blueprints/BP_Rabbit` OtherActor))
  (bind _output_get (set `self.PlayerReference` _asbp_rabbit))
  (`/Engine/EditorBlueprintResources/StandardMacros.DoOnce` false :!label _label
    (:`Completed`
      (if (`/Game/PlatformerDevelopmentKit/Characters/Player/Blueprints/BP_Rabbit.IsHanging?` (`self.PlayerReference`))
        (`/Game/PlatformerDevelopmentKit/Characters/Player/Blueprints/BP_Rabbit.GetOffLedge` (`self.PlayerReference`)))
      (`self.DisableInput` _output_get (`GameplayStatics.GetPlayerController` 0))
      (`self.LaunchCharacter` _playerreference (`KismetMathLibrary.MakeVector` (* _returnvalue_x -500.0) (* _returnvalue_y -500.0) 300.0) true true)
      (set `/Game/PlatformerDevelopmentKit/Characters/Player/Blueprints/BP_Rabbit.CharacterCondition` "NewEnumerator0" _playerreference)
      (`GameplayStatics.SpawnEmitterAtLocation` "/Game/PlatformerDevelopmentKit/Characters/Player/Particles/PS_Impact.PS_Impact" (`self.K2_GetActorLocation` _playerreference))
      (`/Game/PlatformerDevelopmentKit/UI/Widgets/Main_Widget.UpdateHearts` (`/Game/PlatformerDevelopmentKit/Characters/Player/Blueprints/BP_Rabbit.MainWidgetReference` (`self.PlayerReference`)) -1)
      (if (<= (`/Game/PlatformerDevelopmentKit/Characters/Player/Blueprints/BP_Rabbit.CurrentHealth` (`self.PlayerReference`)) 0)
        (set `/Game/PlatformerDevelopmentKit/Characters/Player/Blueprints/BP_Rabbit.CharacterCondition` "NewEnumerator1" _playerreference_2)
        (`self.DisableInput` _playerreference_2 (`GameplayStatics.GetPlayerController` 0))
        (`KismetSystemLibrary.Delay` 0.5)
        (`self.CanBeDamagedAgainPlayer`)
        (if (> (`self.Health`) 0)
          (`KismetSystemLibrary.Delay` 5.0)
          (`self.K2_TeleportTo` (`self.OriginLocation`)))
        (else
          (`KismetSystemLibrary.Delay` 0.5)
          (`self.CanBeDamagedAgainPlayer`))))))

(event `CanBeDamagedAgainSelf`
  (goto _label_2 :!via `Reset`))

(event `self.CapsuleComponent.OnComponentHit`
  (params (HitComponent :type "PrimitiveComponent Object Reference") (OtherActor :type "Actor Object Reference") (OtherComp :type "PrimitiveComponent Object Reference") (NormalImpulse :type "Vector Structure") (Hit :type "HitResult Structure (by ref)"))
  (cast `/Game/PlatformerDevelopmentKit/Interactables/Blueprints/BP_PoopThrown` OtherActor)
  (`/Engine/EditorBlueprintResources/StandardMacros.DoOnce` false :!label _label_2
    (:`Completed`
      (`GameplayStatics.SpawnEmitterAtLocation` "/Game/PlatformerDevelopmentKit/Interactables/Particles/PS_Stars.PS_Stars" (`self.K2_GetActorLocation`))
      (set `self.Health` (- (`self.Health`) 1))
      (if (<= (`self.Health`) 0)
        (set `self.AIState` "NewEnumerator4")
        (`BlackboardComponent.SetValueAsEnum` (`self.PikeeBlackboard`) (`self.AIStateBlackboardKey`) (enumliteral `/Game/PlatformerDevelopmentKit/Characters/Pikee/Blueprints/Enum_AIState` "NewEnumerator4"))
        (else
          (set `self.AIState` "NewEnumerator3")
          (`BlackboardComponent.SetValueAsEnum` (`self.PikeeBlackboard`) (`self.AIStateBlackboardKey`) (enumliteral `/Game/PlatformerDevelopmentKit/Characters/Pikee/Blueprints/Enum_AIState` "NewEnumerator3"))
          (`KismetSystemLibrary.Delay` 0.5)
          (`self.CanBeDamagedAgainSelf`))))))

(fn `UserConstructionScript`)