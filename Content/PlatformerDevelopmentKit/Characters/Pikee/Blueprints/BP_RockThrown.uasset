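; BP_RockThrown is the rock thrown by Pikee that damages the player rabbit on contact.
; A component hit casts to BP_Rabbit and passes a DoOnce, so each rock hurts only once.
; The hit releases any ledge hang, disables input, launches the rabbit backward and up, sets its condition, spawns an impact effect and removes a heart.
; At zero health it switches the rabbit to a second condition.
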(event `self.Rock.OnComponentHit`
  (params (HitComponent :type "PrimitiveComponent Object Reference") (OtherActor :type "Actor Object Reference") (OtherComp :type "PrimitiveComponent Object Reference") (NormalImpulse :type "Vector Structure") (Hit :type "HitResult Structure (by ref)"))
  (bind _playerreference (`self.PlayerReference`))
  (bind _playerreference_2 (`self.PlayerReference`))
  (bind (_returnvalue_x _returnvalue_y) (`KismetMathLibrary.BreakVector` (`self.GetActorForwardVector` (`self.PlayerReference`))))
  (bind _asbp_rabbit (cast `/Game/PlatformerDevelopmentKit/Characters/Player/Blueprints/BP_Rabbit` OtherActor))
  (bind _output_get (set `self.PlayerReference` _asbp_rabbit))
  (`/Engine/EditorBlueprintResources/StandardMacros.DoOnce` false
    (:`Completed`
      (if (`/Game/PlatformerDevelopmentKit/Characters/Player/Blueprints/BP_Rabbit.IsHanging?` (`self.PlayerReference`))
        (`/Game/PlatformerDevelopmentKit/Characters/Player/Blueprints/BP_Rabbit.GetOffLedge` (`self.PlayerReference`)))
      (`self.DisableInput` _output_get (`GameplayStatics.GetPlayerController` 0))
      (`Character.LaunchCharacter` _playerreference (`KismetMathLibrary.MakeVector` (* _returnvalue_x -500.0) (* _returnvalue_y -500.0) 300.0) true true)
      (set `/Game/PlatformerDevelopmentKit/Characters/Player/Blueprints/BP_Rabbit.CharacterCondition` "NewEnumerator0" _playerreference)
      (`GameplayStatics.SpawnEmitterAtLocation` "/Game/PlatformerDevelopmentKit/Characters/Player/Particles/PS_Impact.PS_Impact" (`self.K2_GetActorLocation` _playerreference))
      (`/Game/PlatformerDevelopmentKit/UI/Widgets/Main_Widget.UpdateHearts` (`/Game/PlatformerDevelopmentKit/Characters/Player/Blueprints/BP_Rabbit.MainWidgetReference` (`self.PlayerReference`)) -1)
      (if (<= (`/Game/PlatformerDevelopmentKit/Characters/Player/Blueprints/BP_Rabbit.CurrentHealth` (`self.PlayerReference`)) 0)
        (set `/Game/PlatformerDevelopmentKit/Characters/Player/Blueprints/BP_Rabbit.CharacterCondition` "NewEnumerator1" _playerreference_2)
        (`self.DisableInput` _playerreference_2 (`GameplayStatics.GetPlayerController` 0))
        (`KismetSystemLibrary.Delay` 0.5)))))

(fn `UserConstructionScript`)