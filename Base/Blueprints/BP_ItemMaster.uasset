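; BP_ItemMaster is a base pickup item, collected when BP_Rabbit overlaps its sphere.
; On overlap it disables the sphere's collision responses, spawns a collect particle and adds an Item_Widget carrying its ItemInfo to the player's main widget.
; It then calls PlayItemAnimationWhenObtained, an empty event that child items can override, and destroys itself after the animation length set in ItemInfo.
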(event `self.Sphere.OnComponentBeginOverlap`
  (params (OverlappedComponent :type "PrimitiveComponent Object Reference") (OtherActor :type "Actor Object Reference") (OtherComp :type "PrimitiveComponent Object Reference") (OtherBodyIndex :type Integer) (bFromSweep :type Boolean) (SweepResult :type "HitResult Structure (by ref)"))
  (bind _mainwidgetreference (`/Game/PlatformerDevelopmentKit/Characters/Player/Blueprints/BP_Rabbit.MainWidgetReference` (`self.PlayerReference`)))
  (bind _asbp_rabbit (cast `/Game/PlatformerDevelopmentKit/Characters/Player/Blueprints/BP_Rabbit` OtherActor))
  (set `self.PlayerReference` _asbp_rabbit)
  (`PrimitiveComponent.SetCollisionResponseToAllChannels` (`self.Sphere`) "ECR_Ignore")
  (`GameplayStatics.SpawnEmitterAtLocation` "/Game/PlatformerDevelopmentKit/Interactables/Particles/PS_Collect.PS_Collect" (`SceneComponent.K2_GetComponentLocation` (`self.Sphere`)))
  (bind _returnvalue (`|CreateWidget` "/Game/PlatformerDevelopmentKit/UI/Widgets/Item_Widget.Item_Widget_C"))
  (`/Game/PlatformerDevelopmentKit/UI/Widgets/Item_Widget.SetObtainedItem` _returnvalue (`self.PlayerReference`) (`self.ItemInfo`))
  (`VerticalBox.AddChildToVerticalBox` (`/Game/PlatformerDevelopmentKit/UI/Widgets/Main_Widget.ItemsBox` _mainwidgetreference) _returnvalue)
  (`KismetArrayLibrary.Array_Add` (`/Game/PlatformerDevelopmentKit/UI/Widgets/Main_Widget.ItemWidgets` _mainwidgetreference) _returnvalue)
  (`self.PlayItemAnimationWhenObtained`)
  ;[1 1 1] Animation Length
  (`KismetSystemLibrary.Delay` (`.ObtainedAnimationLength_8_636534904A16C390E01EA7874BC71583` (break `/Game/PlatformerDevelopmentKit/Base/Blueprints/S_ItemInfo` (`self.ItemInfo`))))
  (`self.K2_DestroyActor`))

(event `PlayItemAnimationWhenObtained`)

(fn `UserConstructionScript`)